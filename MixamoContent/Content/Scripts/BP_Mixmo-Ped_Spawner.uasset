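; Spawner actor that populates a level with a set number of Mixamo pedestrians on BeginPlay.
; Each BP_MixamoPed_Base spawns at a random point inside the NavMesh actor's bounding box, without projection onto the navmesh, adjusting for collisions but always spawning.
; A seeded random stream drives both position and the skeletal mesh picked from the Pedestrians array.
; Each pedestrian's AI controller class is set to None after spawning.
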(event EventBeginPlay
  (bind _navmesh (Variables|Default|GetNavMesh))
  (bind _rand (Variables|Default|GetRand))
  (bind _pedestrians (Variables|Default|GetPedestrians))
  (bind (_origin _boxextent) (Collision|GetActorBounds _navmesh false false))
  (Math|Random|SetRandomStreamSeed (Variables|Default|GetRand) (Variables|Default|GetSeed))
  (for _index (range 1 (Variables|Default|GetNumberOfPeds))
    (bind _returnvalue (Game|SpawnActorfromClass "/MixamoContent/Scripts/BP_Mixamo-Ped_Base.BP_Mixamo-Ped_Base_C" (Math|Transform|MakeTransform (Math|Vector|MakeVector (Math|Random|RandomFloatinRangefromStream (- (.x _origin) (.x _boxextent)) (+ (.x _origin) (.x _boxextent)) _rand) (Math|Random|RandomFloatinRangefromStream (- (.y _origin) (.y _boxextent)) (+ (.y _origin) (.y _boxextent)) _rand) (Math|Random|RandomFloatinRangefromStream (- (.z _origin) (.z _boxextent)) (+ (.z _origin) (.z _boxextent)) _rand)) "0, 0, 0" "1,1,1") "AdjustIfPossibleButAlwaysSpawn" 0 0))
    (Class|SkinnedMeshComponent|SetSkeletalMesh (Variables|/Script/Engine.Character|GetMesh _returnvalue) (Utilities|Array|Get(acopy) _pedestrians (Math|Random|RandomIntegerinRangefromStream 0 (Utilities|Array|LastIndex _pedestrians) (Variables|Default|GetRand))) true)
    (Variables|/Script/Engine.Pawn|SetAIControllerClass _returnvalue 0)))

(fn ConstructionScript)