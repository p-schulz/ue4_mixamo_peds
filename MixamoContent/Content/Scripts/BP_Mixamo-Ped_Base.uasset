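; Base pedestrian character Blueprint that turns into a ragdoll when struck by a moving vehicle.
; Its Hit event ignores anything that is not a WheeledVehicle and checks that the vehicle's speed exceeds a small threshold.
; On a valid hit it disables capsule collision and character movement, then switches the mesh to the Ragdoll collision profile and simulates physics on all bodies.
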(event Collision|EventHit
  (params (MyComp :type Primitive%20Component%20Object%20Reference) (Other :type Actor%20Object%20Reference) (OtherComp :type Primitive%20Component%20Object%20Reference) (bSelfMoved :type Boolean) (HitLocation :type Vector :default "0, 0, 0") (HitNormal :type Vector :default "0, 0, 0") (NormalImpulse :type Vector :default "0, 0, 0") (Hit :type Hit%20Result%20Structure%20%28by%20ref%29))
  (bind _mesh (Variables|Character|GetMesh))
  (bind _aswheeled_vehicle (Utilities|Casting|CastToWheeledVehicle Other))
  (if (> (Math|Vector|VectorLength (Transformation|GetVelocity _aswheeled_vehicle)) 3.6)
    (Collision|SetCollisionEnabled (Variables|Collision|GetCapsuleComponent) "NoCollision")
    (Pawn|Components|CharacterMovement|DisableMovement (Variables|Character|GetCharacterMovement))
    (Collision|SetCollisionEnabled _mesh "QueryAndPhysics")
    (Collision|SetCollisionProfileName _mesh "Ragdoll" true :!class /Script/Engine.PrimitiveComponent)
    (Physics|SetSimulatePhysics _mesh true)
    (Class|SkeletalMeshComponent|SetAllBodiesSimulatePhysics _mesh true)))

(fn ConstructionScript)